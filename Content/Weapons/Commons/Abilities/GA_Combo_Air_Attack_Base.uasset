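; GA_Combo_Air_Attack_Base is a gameplay ability base for airborne combo attacks with weapons.
; It can activate only when the character's movement component is not moving on the ground.
; On activation it runs the parent logic, applies the GE_Floating effect to the owner and stores the handle.
; When the ability ends, it removes that effect through the stored handle.
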(event `self.K2_ActivateAbility`
  (`parent.K2_ActivateAbility`)
  (bind _returnvalue (`self.BP_ApplyGameplayEffectToOwner` "/Game/Weapons/Commons/Effects/GE_Floating.GE_Floating_C"))
  (set `self.FloatingEffectHandle` _returnvalue))

(event `self.K2_OnEndAbility`
  (params (bWasCancelled :type Boolean))
  (`parent.K2_OnEndAbility` bWasCancelled)
  (`self.BP_RemoveGameplayEffectFromOwnerWithHandle` (`self.FloatingEffectHandle`)))

(fn `K2_CanActivateAbility`
  (params (ActorInfo :type "GameplayAbilityActorInfo Structure") (Handle :type "GameplayAbilitySpecHandle Structure"))
  (returns (RelevantTags :type "GameplayTagContainer Structure") (ReturnValue :type Boolean))
  (return (struct) (not (`NavMovementComponent.IsMovingOnGround` (`self.GetCharacterMovement`)))))