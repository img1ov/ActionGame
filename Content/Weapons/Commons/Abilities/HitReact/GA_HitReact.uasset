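; Gameplay ability that, triggered by an event, plays a directional hit reaction and applies an impulse to the character.
; The event tag picks a shake, knockback, large knockback or launch montage set; grounded characters get zero impulse except for launches.
; SelectMontage chooses front/back and ground/air montages via dot product, with the section from impact direction.
; For B_Hero_Default, a motion warp target is set at the instigator's location.
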(event `self.K2_ActivateAbilityFromEvent`
  (params (EventData :type "GameplayEventData Structure (by ref)"))
  (bind (_targetmontagesections _sectionfromdirection) (`self.SelectMontage` (`self.TargetCardinals`) (`self.IsOnGround`)))
  (set `self.ImpactTag` EventData_EventTag)
  (set `self.Instigator` EventData_Instigator)
  (set `self.Target` EventData_Target)
  (`|ExecutionSequence`
    (:`then_0`
      (bind _output_get (set `self.HitReactImpuls` (`BulletSystemBlueprintLibrary.GetHitReactImpulseFromEventData` (`self.CurrentEventData`))))
      (set `self.ImpulseVectorDone` (* (`.ImpulseVector` (break `HitReactImpulse` _output_get)) (`.Strength` (break `HitReactImpulse` _output_get)) (`self.ImpulseMultiplierBase`))))
    (:`then_1`
      (set `self.MovementComponent` (`ActCharacter.GetActMovementComponent` (`self.GetActCharacterFromActorInfo`)))
      (set `self.IsOnGround` (`NavMovementComponent.IsMovingOnGround` (`self.MovementComponent`)))
      (`|SwitchGameplayTag` (`self.ImpactTag`)
        (:`Gameplay.HitReact.Shake`
          (set `self.TargetCardinals` (`self.ShakeCardinals`))
          (if (`self.IsOnGround`)
            (set `self.ImpulseVectorDone` (* (`self.ImpulseVectorDone`) (0.0 0.0 0.0)) :!label _label)))
        (:`Gameplay.HitReact.Knockback`
          (set `self.TargetCardinals` (`self.KnockbackCardinals`))
          (if (`self.IsOnGround`)
            (goto _label)))
        (:`Gameplay.HitReact.Knockback.Large`
          (set `self.TargetCardinals` (`self.KnockbackLargeCardinals`))
          (if (`self.IsOnGround`)
            (goto _label)))
        (:`Gameplay.HitReact.Launch`
          (set `self.TargetCardinals` (`self.LaunchCardinals`))
          (if (`self.IsOnGround`)
            _))))
    (:`then_2`
      (`CharacterMovementComponent.AddImpulse` (`self.MovementComponent`) (`self.ImpulseVectorDone`) false))
    (:`then_3`
      (`AT_PlayMontageAndWaitForEvent.CreatePlayMontageAndWaitForEvent` "None" _targetmontagesections (struct) 1.0 _sectionfromdirection
        (:`then`
          (bind _asb_hero_default (cast `/Game/Characters/Heroes/B_Hero_Default` (`self.GetActCharacterFromActorInfo`)))
          (`MotionWarpingComponent.AddOrUpdateWarpTargetFromLocationAndRotation` :`self` (`/Game/Characters/Heroes/B_Hero_Default.MotionWarping` _asb_hero_default) :`WarpTargetName` "FacingTarget" :`TargetLocation` (`Actor.K2_GetActorLocation` (`self.Instigator`))))
        (:`OnCompleted`
          (`self.K2_EndAbility` :!label _label_2))
        (:`OnBlendOut`
          (goto _label_2))
        (:`OnInterrupted`
          (goto _label_2))
        (:`OnCancelled`
          (goto _label_2))))))

(fn `SelectMontage`
  (params (HitReactCardinals :type "/Game/Weapons/Commons/Abilities/HitReact/AbilityStruct_HitReactCardinals Structure") (IsOnGround :type Boolean))
  (returns (TargetMontageSections :type "AnimMontage Object Reference") (SectionFromDirection :type Name))
  (locals (VisualImpactDirection :type Name))
  (bind (_hitreactcardinals_forward _hitreactcardinals_backward _hitreactcardinals_forward_air _hitreactcardinals_backward_air) (break `/Game/Weapons/Commons/Abilities/HitReact/AbilityStruct_HitReactCardinals` (`local.HitReactCardinals`)))
  (bind (_hitreactcardinals_forward_2 _hitreactcardinals_backward_2) (break `/Game/Weapons/Commons/Abilities/HitReact/AbilityStruct_HitReactCardinals` (`local.HitReactCardinals`)))
  (bind _hitreactcardinals_forward_3 (break `/Game/Weapons/Commons/Abilities/HitReact/AbilityStruct_HitReactCardinals` (`local.HitReactCardinals`)))
  (bind (_hitreactcardinals_forward_4 _hitreactcardinals_backward_3 _hitreactcardinals_forward_air_2) (break `/Game/Weapons/Commons/Abilities/HitReact/AbilityStruct_HitReactCardinals` (`local.HitReactCardinals`)))
  (bind (_hitreactimpuls_hitreacttag _hitreactimpuls_visualimpactdirection) (break `HitReactImpulse` (`self.HitReactImpuls`)))
  (`|ExecutionSequence`
    (:`then_0`
      (switch `EImpactDirection` _hitreactimpuls_visualimpactdirection
        (:`Up`
          (set `local.VisualImpactDirection` "Default"))
        (:`Down`
          (set `local.VisualImpactDirection` "Down"))
        (:`Left`
          (set `local.VisualImpactDirection` "Left"))
        (:`Right`
          (set `local.VisualImpactDirection` "Right"))))
    (:`then_1`
      (if (> (`KismetMathLibrary.Dot_VectorVector` (`KismetMathLibrary.Normal` (- (`Actor.K2_GetActorLocation` (`self.Instigator`)) (`Actor.K2_GetActorLocation` (`self.Target`)))) (`Actor.GetActorForwardVector` (`self.Target`))) 0.0)
        (if (`local.IsOnGround`)
          (return _hitreactcardinals_forward_3 (`local.VisualImpactDirection`))
          (else
            (return _hitreactcardinals_forward_air_2 (`local.VisualImpactDirection`))))
        (elif (`local.IsOnGround`)
          (return _hitreactcardinals_backward_2 (`local.VisualImpactDirection`))
          (else
            (return _hitreactcardinals_backward_air (`local.VisualImpactDirection`))))))))