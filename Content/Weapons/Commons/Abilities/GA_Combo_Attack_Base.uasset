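; Base gameplay ability for melee or weapon combo attacks: it commits, plays an attack montage and ends when the montage does.
; Montage gameplay events drive a bullet lifecycle, spawning one at the character's transform, processing its manual hits and destroying it by stored instance ID.
; A recovery event sets the Ability.Phase.Recovery tag, letting movement acceleration end the attack early.
; The tag is cleared when the ability ends.
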(event `self.K2_ActivateAbility`
  (bind _returnvalue (`self.K2_CommitAbility`))
  (if _returnvalue
    (bind (_asynctaskproxy _eventtag) (`AT_PlayMontageAndWaitForEvent.CreatePlayMontageAndWaitForEvent` "None" (`self.MontageToPlay`) (struct :`GameplayTags` (struct :`(TagName` "Event"))))
      (:`OnCompleted`
        (`self.K2_EndAbility` :!label _label))
      (:`OnBlendOut`
        (goto _label))
      (:`OnInterrupted`
        (goto _label))
      (:`OnCancelled`
        (goto _label))
      (:`EventReceived`
        (`self.SwitchOnReceivedEventTag` _eventtag)))))

(event `self.K2_OnEndAbility`
  (params (bWasCancelled :type Boolean))
  (`ActAbilitySystemComponent.K2_SetGameplayTagCount` (`self.GetActAbilitySystemComponentFromActorInfo`) (struct :`TagName` "Ability.Phase.Recovery") 0))

(fn `OnAbilityPhaseRecoveryReceived`
  (params (HasAcceleration :type Boolean))
  (`ActAbilitySystemComponent.K2_SetGameplayTagCount` (`self.GetActAbilitySystemComponentFromActorInfo`) (struct :`TagName` "Ability.Phase.Recovery") 1)
  (if (`local.HasAcceleration`)
    (`self.K2_EndAbility`)))

(fn `OnAccelerationChangedReceived`
  (params (HasAcceleration :type Boolean))
  (if (and (> (`AbilitySystemComponent.GetGameplayTagCount` (`self.GetActAbilitySystemComponentFromActorInfo`) (struct :`TagName` "Ability.Phase.Recovery")) 0) (`local.HasAcceleration`))
    (`self.K2_EndAbility`)))

(fn `OnDestoryBulletReceived`
  (params (InstanceID :type Integer))
  (`BulletBlueprintLibrary.DestroyBullet` InstanceID "Immediate"))

(fn `OnProcessMenuHitReceived`
  (params (InstanceID :type Integer))
  (`BulletBlueprintLibrary.ProcessManualHits` InstanceID))

(fn `OnSpawnBulletReceived`
  (returns (InstanceID :type Integer))
  (bind _returnvalue (`self.GetActCharacterFromActorInfo`))
  (bind _returnvalue_2 (`ActAbilitySystemComponent.K2_SpawnBullet` (`self.GetActAbilitySystemComponentFromActorInfo`) (`self.BulletID`) (make `BulletInitParams` _returnvalue (`Actor.GetTransform` _returnvalue) null (0.0 0.0 0.0) -1 -1 (make `BulletPayload`))))
  (return _returnvalue_2))

(fn `SwitchOnReceivedEventTag`
  (params (EventTag :type "GameplayTag Structure"))
  (locals (HasAcceleration :type Boolean))
  (set `local.HasAcceleration` (`ActCharacterMovementComponent.GetHasAcceleration` (`ActCharacter.GetActMovementComponent` (`self.GetActCharacterFromActorInfo`))))
  (`|SwitchGameplayTag` EventTag
    (:`Event.Movement.AccelerationStateChanged`
      (`self.OnAccelerationChangedReceived` (`local.HasAcceleration`)))
    (:`Event.Ability.Phase.Recovery`
      (`self.OnAbilityPhaseRecoveryReceived` (`local.HasAcceleration`)))
    (:`Event.Bullet.SpawnBullet`
      (bind _instanceid (`self.OnSpawnBulletReceived`))
      (set `self.BulletInstanceID` _instanceid))
    (:`Event.Bullet.ProcessManualHits`
      (`self.OnProcessMenuHitReceived` (`self.BulletInstanceID`)))
    (:`Event.Bullet.DestroyBullet`
      (`self.OnDestoryBulletReceived` (`self.BulletInstanceID`)))))