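; Gameplay ability for the Nodachi launch attack (Attack_Up_Floor_To_Air_02) that lifts the character off the floor into the air.
; On activation it switches movement to Falling, lowers gravity scale, and applies a short world-space upward act motion shaped by a strength curve.
; Ending the ability sets gravity scale back to a fixed default rather than restoring the previous value.
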(event `self.K2_ActivateAbility`
  (bind _returnvalue (`ActCharacter.GetActMovementComponent` (`self.GetActCharacterFromActorInfo`)))
  (`parent.K2_ActivateAbility`)
  (`CharacterMovementComponent.SetMovementMode` _returnvalue "MOVE_Falling" 0)
  (set `CharacterMovementComponent.GravityScale` 0.35 _returnvalue)
  (`AT_ApplyActMotion.ApplyActMotion` "None" "World" (0.0 0.0 1.0) 880.0 0.15 "/Game/Weapons/Nodachi/Abilities/Attack_Launch/Curve_Attack_Up_Floor_To_Air_02.Curve_Attack_Up_Floor_To_Air_02" (`Character.Mesh` (`self.GetActCharacterFromActorInfo`))))

(event `self.K2_OnEndAbility`
  (params (bWasCancelled :type Boolean))
  (`parent.K2_OnEndAbility` bWasCancelled)
  (set `CharacterMovementComponent.GravityScale` 1.0 (`ActCharacter.GetActMovementComponent` (`self.GetActCharacterFromActorInfo`))))