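; GA_Jump is the hero locomotion ability that performs a montage-driven jump.
; It plays the forward jump montage when the character is accelerating without the StrafeMove tag, otherwise the standard one.
; The montage's Jump gameplay event starts the character jump and a "Jumping" ability state, whose end or interruption stops the jump and ends the ability.
; Montage completion, blend out, interruption or cancellation also ends the ability.
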(event `self.K2_ActivateAbility`
  (set `self.MontageToPlay` (select `bool` (and (<= (`AbilitySystemComponent.GetGameplayTagCount` (`self.GetAbilitySystemComponentFromActorInfo`) (struct :`TagName` "Event.Movement.StrafeMove")) 0) (`ActCharacterMovementComponent.GetHasAcceleration` (`ActCharacter.GetActMovementComponent` (`self.GetActCharacterFromActorInfo`)))) :`false` (`self.AM_Jump`) :`true` (`self.AM_Jump_Fwd`)))
  (`AT_PlayMontageAndWaitForEvent.CreatePlayMontageAndWaitForEvent` "None" (`self.MontageToPlay`) (struct :`GameplayTags` (struct :`(TagName` "Event.Movement.Jump")))
    (:`OnCompleted`
      (`self.K2_EndAbility` :!label _label))
    (:`OnBlendOut`
      (goto _label))
    (:`OnInterrupted`
      (goto _label))
    (:`OnCancelled`
      (goto _label))
    (:`EventReceived`
      (`self.CharacterJumpStart`)
      (`AbilityTask_StartAbilityState.StartAbilityState` "Jumping"
        (:`OnStateEnded`
          _)
        (:`OnStateInterrupted`
          _))
      (`self.CharacterJumpStop`)
      (`self.K2_EndAbility`))))