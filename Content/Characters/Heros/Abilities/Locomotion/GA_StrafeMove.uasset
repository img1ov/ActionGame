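; Gameplay ability that puts the hero into a slower strafe movement while its input is held.
; On activation it stops the character orienting rotation to movement and lowers max walk speed.
; When WaitInputRelease fires, it restores movement-facing rotation and the faster speed, then ends the ability.
; A shared SetMovementParams helper writes both values to the avatar's CharacterMovement component.
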(event `self.K2_ActivateAbility`
  (`self.SetMovementParams` false 180.0)
  (`AbilityTask_WaitInputRelease.WaitInputRelease` false
    (:`OnRelease`
      (`self.SetMovementParams` true 500.0)
      (`self.K2_EndAbility`))))

(fn `SetMovementParams`
  (params (OrientRotationToMovement :type Boolean) (MaxWalkSpeed :type "Float (double-precision)"))
  (locals (CharacterMovement :type "ActCharacterMovementComponent Object Reference"))
  (set `local.CharacterMovement` (`ActCharacter.GetActMovementComponent` (`self.GetActCharacterFromActorInfo`)))
  (set `CharacterMovementComponent.bOrientRotationToMovement` (`local.OrientRotationToMovement`) (`local.CharacterMovement`))
  (set `CharacterMovementComponent.MaxWalkSpeed` (`local.MaxWalkSpeed`) (`local.CharacterMovement`)))