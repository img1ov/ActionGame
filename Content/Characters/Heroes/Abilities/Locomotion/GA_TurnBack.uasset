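; Gameplay ability for hero locomotion that plays a turn-back montage through PlayMontageAndWaitForEvent.
; When the montage completes or blends out, it checks the movement component for acceleration and ends if the character has any.
; Without acceleration, it plays a montage again from the same Montage variable and ends on any outcome or received event.
; Interruption or cancellation of the first montage ends the ability immediately.
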(event `self.K2_ActivateAbility`
  (`AT_PlayMontageAndWaitForEvent.PlayMontageAndWaitForEvent` "None" (`self.Montage`)
    (:`OnCompleted`
      (if (not (`ActCharacterMovementComponent.GetHasAcceleration` (`ActCharacter.GetActMovementComponent` (`self.GetActCharacterFromActorInfo`)))) :!label _label
        (`AT_PlayMontageAndWaitForEvent.PlayMontageAndWaitForEvent` "None" (`self.Montage`)
          (:`OnCompleted`
            _)
          (:`OnBlendOut`
            _)
          (:`OnInterrupted`
            _)
          (:`OnCancelled`
            _)
          (:`EventReceived`
            _))
        (`self.K2_EndAbility`)
        (else
          (`self.K2_EndAbility`))))
    (:`OnBlendOut`
      (goto _label))
    (:`OnInterrupted`
      (`self.K2_EndAbility` :!label _label_2))
    (:`OnCancelled`
      (goto _label_2))))